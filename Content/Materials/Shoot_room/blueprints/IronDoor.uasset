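; Iron door actor in the shoot room that swings open with a sound once triggered.
; ChangeIronRotate sets a rotation flag, then starts the audio after a short delay.
; While flagged, Tick adds a fixed, frame-rate-dependent yaw step until the mesh's world yaw passes zero from its commented -90° default.
; It then stops the audio on every tick, as the flag is never cleared.
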(event `self.ReceiveTick`
  (params (DeltaSeconds :type "Float (single-precision)"))
  ;[0.1302 0.1302 0.1302] Por padrão, a porta de ferro está com -90° de rotação em Z. Ao chegar em 0, ela irá parar de abrir, como faz o código abaixo:
  (if (`self.makeIronDoorRotate`)
    (if (<= (.yaw (`SceneComponent.K2_GetComponentRotation` (`self.ironDoorMesh`))) 0.0)
      (`self.K2_AddActorLocalRotation` (`KismetMathLibrary.MakeRotator` 0.0 0.0 0.5))
      (else
        (`AudioComponent.Stop` (`self.Audio`))))))

(event `ChangeIronRotate`
  (set `self.makeIronDoorRotate` true)
  (`KismetSystemLibrary.Delay` 1.0)
  (`AudioComponent.Play` (`self.Audio`) 0.0))

(fn `UserConstructionScript`)