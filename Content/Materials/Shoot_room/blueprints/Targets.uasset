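; Shooting-room target set with three targets (left, center, right) that fall when hit and, once all are down, unlock the room.
; Each hit box turns on physics and gravity for its target and sets a fallen flag, then runs a shared all-three check.
; On success it finds tagged actors to zero the room's spot and point lights and swap the red/green indicator materials, then calls IronDoor's rotate event to open the door.
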(event `self.RIGHT_BOX.OnComponentHit`
  (params (HitComponent :type "PrimitiveComponent Object Reference") (OtherActor :type "Actor Object Reference") (OtherComp :type "PrimitiveComponent Object Reference") (NormalImpulse :type "Vector Structure") (Hit :type "HitResult Structure (by ref)"))
  (bind _right_target (`self.RIGHT_TARGET`))
  (`PrimitiveComponent.SetSimulatePhysics` _right_target true)
  (`PrimitiveComponent.SetEnableGravity` _right_target true)
  (bind _output_get (set `self.rightTargetAlreadyFallen` true))
  (if (and _output_get (stale `self.CENTER_BOX.OnComponentHit` _output_get) (stale `self.LEFT_BOX.OnComponentHit` _output_get)) :!label _label
    ;[0.1823 0.1823 0.1823] Apagando luzes após o usuário acertar todos os alvos
    (bind _outactors (`GameplayStatics.GetAllActorsWithTag` "LuzSala"))
    (for _array_element _outactors
      (bind _asspot_light (cast `SpotLight` _array_element)
        (:`then`
          (`LightComponent.SetIntensity` (`SpotLight.SpotLightComponent` _asspot_light) 0.0))
        (:`CastFailed`
          (bind _aspoint_light (cast `PointLight` _array_element)
            (:`then`
              (`LightComponent.SetIntensity` (`PointLight.PointLightComponent` _aspoint_light) 0.0))
            (:`CastFailed`
              (`KismetSystemLibrary.PrintString` "Falha ao converter para POINT LIGHT" false true (struct :`R` 1.0 :`B` 0.035135 :`A` 1.0) 10.0))))))
    ;[0.1667 0.1667 0.1667] apagando LED vermelho, acendendo o LED verde e abrindo a porta de ferro após o jogador atirar e acertar todos os alvos
    (bind _outactors_2 (`GameplayStatics.GetAllActorsWithTag` "greenCube"))
    (for _array_element_2 _outactors_2
      (bind _asstatic_mesh_actor (cast `StaticMeshActor` _array_element_2)
        (:`then`
          (`PrimitiveComponent.SetMaterial` (`StaticMeshActor.StaticMeshComponent` _asstatic_mesh_actor) 0 "/Game/Materials/Shoot_room/materials/green.green"))
        (:`CastFailed`
          (`KismetSystemLibrary.PrintString` "Falha ao tentar converter para StaticMeshActor" true true (struct :`R` 1.0 :`B` 0.089962 :`A` 1.0)))))
    (bind _outactors_3 (`GameplayStatics.GetAllActorsWithTag` "redCube"))
    (for _array_element_3 _outactors_3
      (bind _asstatic_mesh_actor_2 (cast `StaticMeshActor` _array_element_3)
        (:`then`
          (`PrimitiveComponent.SetMaterial` (`StaticMeshActor.StaticMeshComponent` _asstatic_mesh_actor_2) 0 "/Game/Materials/Shoot_room/materials/wall_material.wall_material"))
        (:`CastFailed`
          (`KismetSystemLibrary.PrintString` "Falha ao tentar converter para StaticMeshActor 2" true true (struct :`R` 1.0 :`B` 0.089962 :`A` 1.0)))))
    ;[0.2865 0.2865 0.2865] Acionando evento para abrir a porta via blueprint 'IronDoor'
    (bind _returnvalue (`GameplayStatics.GetActorOfClass` "/Game/Materials/Shoot_room/blueprints/IronDoor.IronDoor_C"))
    (`/Game/Materials/Shoot_room/blueprints/IronDoor.ChangeIronRotate` _returnvalue)
    (`KismetSystemLibrary.PrintString` "CHAMOU O EVENTO DA PORTA" false true (struct :`R` 0.414964 :`G` 1.0 :`A` 1.0))))

(event `self.CENTER_BOX.OnComponentHit`
  (params (HitComponent :type "PrimitiveComponent Object Reference") (OtherActor :type "Actor Object Reference") (OtherComp :type "PrimitiveComponent Object Reference") (NormalImpulse :type "Vector Structure") (Hit :type "HitResult Structure (by ref)"))
  (bind _center_target (`self.CENTER_TARGET`))
  (`PrimitiveComponent.SetSimulatePhysics` _center_target true)
  (`PrimitiveComponent.SetEnableGravity` _center_target true)
  (bind _output_get (set `self.centerTargetAlreadyFallen` true))
  (goto _label))

(event `self.LEFT_BOX.OnComponentHit`
  (params (HitComponent :type "PrimitiveComponent Object Reference") (OtherActor :type "Actor Object Reference") (OtherComp :type "PrimitiveComponent Object Reference") (NormalImpulse :type "Vector Structure") (Hit :type "HitResult Structure (by ref)"))
  (bind _left_target (`self.LEFT_TARGET`))
  (`PrimitiveComponent.SetSimulatePhysics` _left_target true)
  (`PrimitiveComponent.SetEnableGravity` _left_target true)
  (bind _output_get (set `self.leftTargetAlreadyFallen` true))
  (goto _label))

(fn `UserConstructionScript`)