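; TextEquipWeapon is a trigger actor that shows a weapon-equip text prompt when something enters its Box.
; It starts hidden with collision left on, reveals itself on Box overlap by any actor, and hides again on actor end overlap.
; When BP_FirstPersonCharacter enters, it hands the character and itself to the first RotateWeapon found in the level.
; Debug prints trace each step, and disconnected GamesVariables nodes remain from testing.
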(event `self.ReceiveActorBeginOverlap`
  (params (OtherActor :type "Actor Object Reference")))

(event `self.Box.OnComponentBeginOverlap`
  (params (OverlappedComponent :type "PrimitiveComponent Object Reference") (OtherActor :type "Actor Object Reference") (OtherComp :type "PrimitiveComponent Object Reference") (OtherBodyIndex :type Integer) (bFromSweep :type Boolean) (SweepResult :type "HitResult Structure (by ref)"))
  (`KismetSystemLibrary.PrintString` "ENTROUUU" true true (struct :`R` 0.393641 :`G` 1.0 :`A` 1.0))
  (`self.SetActorHiddenInGame` self false)
  (`self.SetActorEnableCollision` true)
  (`KismetSystemLibrary.PrintString` "TEXTO APARECEU" true true (struct :`R` 0.545985 :`G` 1.0 :`A` 1.0))
  (bind _asbp_first_person_character (cast `/Game/FirstPerson/Blueprints/BP_FirstPersonCharacter` OtherActor)
    (:`then`
      (bind _outactors (`GameplayStatics.GetAllActorsOfClass` "/Game/Materials/Shoot_room/blueprints/RotateWeapon.RotateWeapon_C"))
      (bind _asrotate_weapon (cast `/Game/Materials/Shoot_room/blueprints/RotateWeapon` (`|GetArrayItem` _outactors))
        (:`then`
          (set `/Game/Materials/Shoot_room/blueprints/RotateWeapon.FirstPersonCharacterReference` _asbp_first_person_character _asrotate_weapon)
          (set `/Game/Materials/Shoot_room/blueprints/RotateWeapon.TextEquipInstructionRef` self _asrotate_weapon)
          (`KismetSystemLibrary.PrintString` "TextEquipWeapon foi enviado para RotateWeapon!" false true (struct :`R` 0.40282 :`G` 1.0 :`B` 0.004949 :`A` 1.0)))
        (:`CastFailed`
          (`KismetSystemLibrary.PrintString` "Falha ao tentar converter To RotateWeapon" true true (struct :`R` 1.0 :`G` 0.539124 :`A` 1.0)))))
    (:`CastFailed`
      (`KismetSystemLibrary.PrintString` "Falha ao tentar converter To BP_FirstPersonCharacter" true true (struct :`R` 1.0 :`G` 0.211753 :`B` 0.021443 :`A` 1.0)))))

(event `self.ReceiveActorEndOverlap`
  (params (OtherActor :type "Actor Object Reference"))
  (`self.SetActorHiddenInGame` self true :!label _label)
  (`self.SetActorEnableCollision` true)
  (`KismetSystemLibrary.PrintString` "TEXTO OCULTADO" true true (struct :`G` 0.592601 :`B` 1.0 :`A` 1.0)))

(event `self.ReceiveBeginPlay`
  (goto _label))

(event `self.Box.OnComponentEndOverlap`
  (params (OverlappedComponent :type "PrimitiveComponent Object Reference") (OtherActor :type "Actor Object Reference") (OtherComp :type "PrimitiveComponent Object Reference") (OtherBodyIndex :type Integer)))

(fn `UserConstructionScript`)